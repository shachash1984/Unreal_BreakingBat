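; Blue gem pickup worth one score point, built on a parent class and destroyed when collected.
; The construction script runs the parent's, then sets the score value.
; From BeginPlay, the FloatingAnimation timeline rewrites the mesh's relative transform each update, adding its track value to actor Z, offsetting actor roll and forcing a fixed scale.
; An unconnected material parameter node never runs.
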(event EventOnCollected
  (Actor|DestroyActor))

(event EventBeginPlay
  (bind _returnvalue (Transformation|GetActorTransform))
  (bind _newtrack_0 (Timeline|FloatingAnimation Play)
    (:Update
      (Transformation|SetRelativeTransform (Variables|Default|GetPickupMesh) (Math|Transform|MakeTransform (Math|Vector|MakeVector (.x (.location _returnvalue)) (.y (.location _returnvalue)) (+ _newtrack_0 (.z (.location _returnvalue)))) (Math|Rotator|MakeRotator (+ (.roll (.rotation _returnvalue)) 1.0) 0.0 0.0) "5.000000,5.000000,5.000000") false false))))

(fn ConstructionScript
  (|CallParentFunction)
  (Class|Pickup|SetScoreValue 1))