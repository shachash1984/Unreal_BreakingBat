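; Dialogue handler for Boris's gem-collecting quest, driving the dialogue widget and the final end screen.
; The Interact input toggles the dialogue with timeline opacity fades, branching on a quest-state enum from start through in-quest to end.
; Text depends on whether the character has an interactable actor and whether the player state reports all gems collected.
; Delivering the gems shows the end screen and mouse cursor after a short delay.
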(event EventBeginPlay
  (Variables|Default|SetDialogueState "EGameStart")
  (bind _asbreaking_bat_character (Utilities|Casting|CastToBreakingBatCharacter (Game|GetPlayerCharacter 0)))
  (bind _output_get (Variables|Default|SetBBCharacterRef _asbreaking_bat_character))
  (bind _returnvalue (Class|BreakingBatCharacter|GetBBPlayerState _output_get))
  (Variables|Default|SetPlayerStateRef _returnvalue))

(event EventEndPlay
  (params (EndPlayReason :type EEndPlayReason%20Enum :default "Destroyed"))
  (Variables|Default|SetDialogVisible false))

(event EventTick
  (params (DeltaSeconds :type Float%20%28single-precision%29)))

(event Input|ActionEvents|InputActionInteract
  (params (Key :type Key%20Structure))
  (bind _returnvalue (Game|GetPlayerController 0))
  (:Pressed
    (switch Utilities|FlowControl|Switch|SwitchonEDialoguesENUM (Variables|Default|GetDialogueState)
      (:EGameStart
        (if (Variables|Default|GetDialogVisible)
          ;[1 1 1] Handle Quest Start
          ;;[1 1 1] HideDialogue
          (Variables|Default|SetDialogVisible false)
          (bind _newtrack_0 (Timeline|FadeoutDialogue ReverseFromEnd)
            (:Update
              (Widget|SetRenderOpacity (Variables|Default|GetWBPDialougeRef) _newtrack_0)
              (Utilities|FlowControl|Delay 0.5)
              (Widget|RemovefromParent (Variables|Default|GetWBPDialougeRef))))
          (else
            ;;[1 1 1] ShowDialogue
            (Utilities|IsValid (Variables|Default|GetWBPDialougeRef)
              (:Is%20Valid
                _)
              (:Is%20Not%20Valid
                (bind _returnvalue_2 (UserInterface|CreateWidget "/Game/UMG/WBP_Dialogue.WBP_Dialogue_C" (Game|GetPlayerController 0)))
                (Variables|Default|SetWBPDialougeRef _returnvalue_2)))
            (Widget|SetRenderOpacity (Variables|Default|GetWBPDialougeRef) 0.0)
            (UserInterface|Viewport|AddtoViewport (Variables|Default|GetWBPDialougeRef) 0)
            (Variables|Default|SetDialogVisible true)
            (bind _newtrack_0_2 (Timeline|FadeInDialogue PlayFromStart)
              (:Update
                (Widget|SetRenderOpacity (Variables|Default|GetWBPDialougeRef) _newtrack_0_2)
                (bind _returnvalue_3 (Class|BreakingBatCharacter|GetInteractableActor (Variables|Default|GetBBCharacterRef)))
                (Utilities|IsValid _returnvalue_3
                  (:Is%20Valid
                    (Default|SetDialogueText (Variables|Default|GetWBPDialougeRef) "Hello my sweet child! can you help me find all my beloved gems?")
                    (Default|SetHeadlineText (Variables|Default|GetWBPDialougeRef) "Boris")
                    (Variables|Default|SetDialogueState "EInQuest"))
                  (:Is%20Not%20Valid
                    (Default|SetDialogueText (Variables|Default|GetWBPDialougeRef) "Go And Find Boris")
                    (Default|SetHeadlineText (Variables|Default|GetWBPDialougeRef)))))))))
      (:EInQuest
        (bind _returnvalue_4 (Class|BreakingBatPlayerState|CollectedAllGems (Variables|Default|GetPlayerStateRef)))
        (if _returnvalue_4
          (Variables|Default|SetDialogueState "EFinishedQuest")
          (if (Variables|Default|GetDialogVisible) :!label _label
            ;[1 1 1] Handle Quest End
            ;;[1 1 1] HideDialogue
            (Variables|Default|SetDialogVisible false)
            (bind _newtrack_0_3 (Timeline|Timeline_3 ReverseFromEnd)
              (:Update
                (Widget|SetRenderOpacity (Variables|Default|GetWBPDialougeRef) _newtrack_0_3)
                (Widget|RemovefromParent (Variables|Default|GetWBPDialougeRef))))
            (else
              ;;[1 1 1] ShowDialogue
              (Utilities|IsValid (Variables|Default|GetWBPDialougeRef)
                (:Is%20Valid
                  _)
                (:Is%20Not%20Valid
                  (bind _returnvalue_5 (UserInterface|CreateWidget "/Game/UMG/WBP_Dialogue.WBP_Dialogue_C" (Game|GetPlayerController 0)))
                  (Variables|Default|SetWBPDialougeRef _returnvalue_5)))
              (Widget|SetRenderOpacity (Variables|Default|GetWBPDialougeRef) 0.0)
              (UserInterface|Viewport|AddtoViewport (Variables|Default|GetWBPDialougeRef) 0)
              (Variables|Default|SetDialogVisible true)
              (bind _newtrack_0_4 (Timeline|Timeline_2 PlayFromStart)
                (:Update
                  (Widget|SetRenderOpacity (Variables|Default|GetWBPDialougeRef) _newtrack_0_4)
                  (bind _returnvalue_6 (Class|BreakingBatCharacter|GetInteractableActor (Variables|Default|GetBBCharacterRef)))
                  (Utilities|IsValid _returnvalue_6
                    (:Is%20Valid
                      (Default|SetDialogueText (Variables|Default|GetWBPDialougeRef) "Yey! You Brought me all of my beloved Gems! Thank you child!")
                      (Default|SetHeadlineText (Variables|Default|GetWBPDialougeRef) "Boris")
                      (Utilities|FlowControl|Delay 2.0)
                      (Utilities|IsValid (Variables|Default|GetWBP_EndScreen)
                        (:Is%20Valid
                          _)
                        (:Is%20Not%20Valid
                          (bind _returnvalue_7 (UserInterface|CreateWidget "/Game/UMG/WBP_EndScreen.WBP_EndScreen_C" _returnvalue))
                          (Variables|Default|SetWBP_EndScreen _returnvalue_7)))
                      (UserInterface|Viewport|AddtoViewport (Variables|Default|GetWBP_EndScreen) 100)
                      (Variables|/Script/Engine.PlayerController|SetbShowMouseCursor _returnvalue true))
                    (:Is%20Not%20Valid
                      (Default|SetDialogueText (Variables|Default|GetWBPDialougeRef) "You Collected all the gems! now go and give them to Boris")
                      (Default|SetHeadlineText (Variables|Default|GetWBPDialougeRef))))))))
          (elif (Variables|Default|GetDialogVisible)
            ;[1 1 1] Handle In Quest
            ;;[1 1 1] HideDialogue
            (Variables|Default|SetDialogVisible false)
            (bind _newtrack_0_5 (Timeline|Timeline_1 ReverseFromEnd)
              (:Update
                (Widget|SetRenderOpacity (Variables|Default|GetWBPDialougeRef) _newtrack_0_5)
                (Widget|RemovefromParent (Variables|Default|GetWBPDialougeRef))))
            (else
              ;;[1 1 1] ShowDialogue
              (Utilities|IsValid (Variables|Default|GetWBPDialougeRef)
                (:Is%20Valid
                  _)
                (:Is%20Not%20Valid
                  (bind _returnvalue_8 (UserInterface|CreateWidget "/Game/UMG/WBP_Dialogue.WBP_Dialogue_C" (Game|GetPlayerController 0)))
                  (Variables|Default|SetWBPDialougeRef _returnvalue_8)))
              (Widget|SetRenderOpacity (Variables|Default|GetWBPDialougeRef) 0.0)
              (UserInterface|Viewport|AddtoViewport (Variables|Default|GetWBPDialougeRef) 0)
              (Variables|Default|SetDialogVisible true)
              (bind _newtrack_0_6 (Timeline|Timeline_0 PlayFromStart)
                (:Update
                  (Widget|SetRenderOpacity (Variables|Default|GetWBPDialougeRef) _newtrack_0_6)
                  (bind _returnvalue_9 (Class|BreakingBatCharacter|GetInteractableActor (Variables|Default|GetBBCharacterRef)))
                  (Utilities|IsValid _returnvalue_9
                    (:Is%20Valid
                      _)
                    (:Is%20Not%20Valid
                      _))
                  (Default|SetDialogueText (Variables|Default|GetWBPDialougeRef) "Gather all of the Blue Gems and deliver them to Boris. Golden cups replenish health. And remember, stay away from the fire!")
                  (Default|SetHeadlineText (Variables|Default|GetWBPDialougeRef))))))))
      (:EFinishedQuest
        (goto _label)))))

(fn ConstructionScript)